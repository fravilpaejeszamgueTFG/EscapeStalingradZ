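; BP_CharacterToFree is a character to be freed on the Grid, shown as one of Becker, Dasha, Katyusha or Til.
; Shortly after BeginPlay it applies its material, then asks the Grid actor to set its start location.
; SetMaterialCharacter picks the mesh material from CharacterChosen, falling back to Til for any other value.
; The SetImage event reapplies that material on demand.
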(event EventBeginPlay
  (Utilities|FlowControl|Delay 0.2)
  (CallFunction|SetMaterialCharacter)
  (bind _returnvalue (Actor|GetActorOfClass "/Script/EscapeStalingradZ.Grid"))
  (Class|Grid|SetCharactertoFreeStartLocation _returnvalue self))

(event EventTick
  (params (DeltaSeconds :type Float%20%28single-precision%29)))

(event Collision|EventActorBeginOverlap
  (params (OtherActor :type Actor%20Object%20Reference)))

(event EventSetImage
  (CallFunction|SetMaterialCharacter))

(fn ConstructionScript)

(fn SetMaterialCharacter
  (bind _characterchosen (Variables|Default|GetcharacterChosen))
  (if (Utilities|Enum|Equal(Enum) _characterchosen "Becker")
    (Rendering|Material|SetMaterial (Variables|Character|GetMesh) 0 "/Game/art/materials/M_Becker.M_Becker")
    (elif (Utilities|Enum|Equal(Enum) _characterchosen "Dasha")
      (Rendering|Material|SetMaterial (Variables|Character|GetMesh) 0 "/Game/art/materials/M_Dasha.M_Dasha")
      (elif (Utilities|Enum|Equal(Enum) _characterchosen "Katyusha")
        (Rendering|Material|SetMaterial (Variables|Character|GetMesh) 0 "/Game/art/materials/M_Katyusha.M_Katyusha")
        (else
          (Rendering|Material|SetMaterial (Variables|Character|GetMesh) 0 "/Game/art/materials/M_Til.M_Til"))))))