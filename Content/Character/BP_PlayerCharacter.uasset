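; Player character Blueprint that applies the look of the selected character and registers itself with the level's Grid on spawn.
; On BeginPlay, SetMaterialCharacter picks the mesh material from CharacterChosen (Becker, Dasha, Katyusha, with Til as the fallback).
; It then finds the Grid actor in the world and calls SetPlayerStartLocation on it, passing itself.
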(event EventBeginPlay
  (CallFunction|SetMaterialCharacter)
  (bind _returnvalue (Actor|GetActorOfClass "/Script/EscapeStalingradZ.Grid"))
  (bind _output_get (Variables|Default|Setgrid _returnvalue))
  (Class|Grid|SetPlayerStartLocation _output_get self))

(fn ConstructionScript)

(fn SetMaterialCharacter
  (bind _characterchosen (Variables|Default|GetcharacterChosen))
  (if (Utilities|Enum|Equal(Enum) _characterchosen "Becker")
    (Rendering|Material|SetMaterial (Variables|Character|GetMesh) 0 "/Game/art/materials/M_Becker.M_Becker")
    (elif (Utilities|Enum|Equal(Enum) _characterchosen "Dasha")
      (Rendering|Material|SetMaterial (Variables|Character|GetMesh) 0 "/Game/art/materials/M_Dasha.M_Dasha")
      (elif (Utilities|Enum|Equal(Enum) _characterchosen "Katyusha")
        (Rendering|Material|SetMaterial (Variables|Character|GetMesh) 0 "/Game/art/materials/M_Katyusha.M_Katyusha")
        (else
          (Rendering|Material|SetMaterial (Variables|Character|GetMesh) 0 "/Game/art/materials/M_Til.M_Til"))))))