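; BP_DoorIcon is an actor that displays a door icon through a BP_WDoor widget held in a widget component.
; After a short delay on BeginPlay, it finds and caches the widget if needed, then calls ChangeImage with its rotated and open states.
; SetImage repeats the same update on demand, skipping the delay.
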(event EventBeginPlay
  (Utilities|FlowControl|Delay 0.2)
  (Utilities|IsValid (Variables|Default|Getdoor)
    (:Is%20Valid
      _)
    (:Is%20Not%20Valid
      (bind _asbp_wdoor (Utilities|Casting|CastToBP_WDoor (UserInterface|GetWidget (Variables|Default|GetWidget))))
      (Variables|Default|Setdoor _asbp_wdoor)))
  (Default|ChangeImage (Variables|Default|Getdoor) (Variables|Default|GetisRotated) (Variables|Default|GetisOpen)))

(event EventSetImage
  (Utilities|IsValid (Variables|Default|Getdoor)
    (:Is%20Valid
      _)
    (:Is%20Not%20Valid
      (bind _asbp_wdoor (Utilities|Casting|CastToBP_WDoor (UserInterface|GetWidget (Variables|Default|GetWidget))))
      (Variables|Default|Setdoor _asbp_wdoor)))
  (Default|ChangeImage (Variables|Default|Getdoor) (Variables|Default|GetisRotated) (Variables|Default|GetisOpen)))

(fn ConstructionScript)