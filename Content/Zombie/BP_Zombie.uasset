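; BP_Zombie is a zombie Blueprint whose body material reflects its type.
; On BeginPlay it calls SetMaterialZombie, which checks TypeOfZombie through nested branches and sets the first material slot of the Mesh.
; Beta, Armoured and Kugelfisch each get their own material, while any other type falls back to the Alpha material.
; The construction script is empty, so the material is applied only at runtime.
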(event EventBeginPlay
  (CallFunction|SetMaterialZombie))

(fn ConstructionScript)

(fn SetMaterialZombie
  (bind _typeofzombie (Variables|Default|GettypeOfZombie))
  (if (Utilities|Enum|Equal(Enum) _typeofzombie "Beta")
    (Rendering|Material|SetMaterial (Variables|Character|GetMesh) 0 "/Game/Art/Materials/M_Beta.M_Beta")
    (elif (Utilities|Enum|Equal(Enum) _typeofzombie "Armoured")
      (Rendering|Material|SetMaterial (Variables|Character|GetMesh) 0 "/Game/Art/Materials/M_Armored.M_Armored")
      (elif (Utilities|Enum|Equal(Enum) _typeofzombie "Kugelfisch")
        (Rendering|Material|SetMaterial (Variables|Character|GetMesh) 0 "/Game/Art/Materials/M_Kugelfisch.M_Kugelfisch")
        (else
          (Rendering|Material|SetMaterial (Variables|Character|GetMesh) 0 "/Game/Art/Materials/M_Alpha.M_Alpha"))))))